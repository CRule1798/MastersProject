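; BP_HeartShield is a level-ending trigger actor that handles a heart pickup or placement, a door and an exit cutscene.
; BeginPlay toggles the hearts and particle visibility and shows a half-heart widget.
; Overlapping Box toggles the hearts again, removes the widget, toggles particles, then slides the door on a timeline after a delay.
; Overlapping BoxDoor shows a fullscreen cutscene widget and opens MainMenu after a hardcoded delay.
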(event OnComponentBeginOverlap(Box)
  (params (OverlappedComponent :type Primitive%20Component%20Object%20Reference) (OtherActor :type Actor%20Object%20Reference) (OtherComp :type Primitive%20Component%20Object%20Reference) (OtherBodyIndex :type Integer) (bFromSweep :type Boolean) (SweepResult :type Hit%20Result%20Structure%20%28by%20ref%29))
  (Rendering|ToggleVisibility (Variables|Default|GetFullHearts) false)
  (Widget|RemovefromParent (Variables|Default|GetHeartUi))
  (Utilities|FlowControl|Delay 0.1)
  (Rendering|ToggleVisibility (Variables|Default|GetNS_BlowingParticles1) false)
  (Utilities|FlowControl|Delay 2.0)
  (bind _newtrack_0 (Timeline|DoorAnim Play)
    (:Update
      (Transformation|SetRelativeLocation (Variables|Default|GetDoor) _newtrack_0 false false))))

(event OnComponentBeginOverlap(BoxDoor)
  (params (OverlappedComponent :type Primitive%20Component%20Object%20Reference) (OtherActor :type Actor%20Object%20Reference) (OtherComp :type Primitive%20Component%20Object%20Reference) (OtherBodyIndex :type Integer) (bFromSweep :type Boolean) (SweepResult :type Hit%20Result%20Structure%20%28by%20ref%29))
  (bind _returnvalue (UserInterface|CreateWidget "/Game/Blueprints/BPW_FullscreenCutscene.BPW_FullscreenCutscene_C"))
  (UserInterface|Viewport|AddtoViewport _returnvalue 0)
  (Utilities|FlowControl|Delay 16.46)
  (Game|OpenLevel(byName) "MainMenu"))

(event EventBeginPlay
  (Rendering|ToggleVisibility (Variables|Default|GetFullHearts) false)
  (Rendering|ToggleVisibility (Variables|Default|GetNS_BlowingParticles1) false)
  (bind _returnvalue (UserInterface|CreateWidget "/Game/Blueprints/BPW_HalfHeart_05.BPW_HalfHeart_05_C"))
  (bind _output_get (Variables|Default|SetHeartUi _returnvalue))
  (UserInterface|Viewport|AddtoViewport _output_get 0))

(fn ConstructionScript)