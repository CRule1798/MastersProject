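; A keycard-locked sliding door that opens for a first-person character carrying the matching keycard.
; On box overlap, it scans the character's Keycards boolean array for a true entry at index KeycardValue, then enables input and plays the Door_anim timeline.
; The timeline drives the mesh's relative location, and pressing E while input is enabled also plays it.
; Leaving the box disables input; nothing reverses the door.
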(event OnComponentBeginOverlap(Box)
  (params (OverlappedComponent :type Primitive%20Component%20Object%20Reference) (OtherActor :type Actor%20Object%20Reference) (OtherComp :type Primitive%20Component%20Object%20Reference) (OtherBodyIndex :type Integer) (bFromSweep :type Boolean) (SweepResult :type Hit%20Result%20Structure%20%28by%20ref%29))
  (bind _asbp_first_person_character (Utilities|Casting|CastToBP_FirstPersonCharacter OtherActor))
  (for (_array_element _array_index) (Variables|/Game/FirstPerson/Blueprints/BP_FirstPersonCharacter.BP_FirstPersonCharacter_C|GetKeycards _asbp_first_person_character)
    (if (and _array_element (== _array_index (Variables|Default|GetKeycard_Value)))
      (Input|EnableInput (Game|GetPlayerController 0))
      (bind _doorsliding (Timeline|Door_anim Play)
        (:Update
          (Transformation|SetRelativeLocation (Variables|Default|GetDoor_Mesh) _doorsliding false false))))))

(event OnComponentEndOverlap(Box)
  (params (OverlappedComponent :type Primitive%20Component%20Object%20Reference) (OtherActor :type Actor%20Object%20Reference) (OtherComp :type Primitive%20Component%20Object%20Reference) (OtherBodyIndex :type Integer))
  (Utilities|Casting|CastToBP_FirstPersonCharacter OtherActor)
  (Input|DisableInput (Game|GetPlayerController 0)))

(event Input|KeyboardEvents|E
  (params (Key :type Key%20Structure :default "None"))
  (:Pressed
    (bind _doorsliding (Timeline|Door_anim Play)
      (:Update
        (Transformation|SetRelativeLocation (Variables|Default|GetDoor_Mesh) _doorsliding false false)))))

(fn ConstructionScript)